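; BP_PuzzleController opens a board puzzle when the player triggers a door interaction and reveals an effect once it is completed.
; It binds to the player InteractionComponent's door event and, if CanBeSolved, shows a UW_Board widget with a back-reference to itself and UI-only input.
; OnPuzzleCompleted removes the board, restores game input and makes the AffectedActor's Niagara component visible.
; An unconnected node for clearing CanBeSolved never runs.
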(event Custom|OnDoorInteraction_Event
  (bind _returnvalue (Game|GetPlayerController 0))
  (if (Variables|Default|GetCanBeSolved)
    (bind _returnvalue_2 (UserInterface|CreateWidget "/Game/Blueprints/UW/UW_Board.UW_Board_C"))
    (bind _output_get (Variables|Default|SetBoardUW _returnvalue_2))
    (Variables|/Game/Blueprints/UW/UW_Board.UW_Board_C|SetPuzzleController _output_get self)
    (UserInterface|Viewport|AddtoViewport _returnvalue_2 0)
    (Input|SetInputModeUIOnly _returnvalue _returnvalue_2 "DoNotLock" true)
    (Variables|/Script/Engine.PlayerController|SetbShowMouseCursor _returnvalue true)))

(event Custom|OnPuzzleCompleted
  (Widget|RemovefromParent (Variables|Default|GetBoardUW))
  (Input|SetInputModeGameOnly (Game|GetPlayerController 0) true)
  (Rendering|SetVisibility (Actor|GetComponentbyClass (Variables|Default|GetAffectedActor) "/Script/Niagara.NiagaraComponent") true false))

(event EventBeginPlay
  (EventDispatchers|AssignOnDoorInteraction (Actor|GetComponentbyClass (Game|GetPlayerCharacter 0) "/Script/GraphicAdventure_UE.InteractionComponent") (delegate Custom|OnDoorInteraction_Event)))

(fn ConstructionScript)