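; BP_OverlayController shows and hides a UW_PauseMenu widget based on the player's proximity to interactables.
; On BeginPlay it creates the widget once and binds to the close and away events of the player character's InteractionComponent.
; The close event adds the widget to the viewport and the away event removes it, each printing a debug message.
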(event Custom|CloseToInteractable_Event
  (UserInterface|Viewport|AddtoViewport (stale EventBeginPlay _returnvalue_3) 0)
  (Development|PrintText "ADD"))

(event Custom|AwayFromInteractable_Event
  (Widget|RemovefromParent (stale EventBeginPlay _returnvalue_3))
  (Development|PrintText "REMOVE"))

(event EventBeginPlay
  (bind _returnvalue (Game|GetPlayerCharacter 0))
  (bind _returnvalue_2 (Actor|GetComponentbyClass _returnvalue "/Script/GraphicAdventure_UE.InteractionComponent"))
  (Utilities|FlowControl|Sequence
    (:then_0
      (bind _returnvalue_3 (UserInterface|CreateWidget "/Game/Blueprints/UW/UW_PauseMenu.UW_PauseMenu_C")))
    (:then_1
      (EventDispatchers|AssignClosetoInteractable _returnvalue_2 (delegate Custom|CloseToInteractable_Event)))
    (:then_2
      (EventDispatchers|AssignAwayfromInteractable _returnvalue_2 (delegate Custom|AwayFromInteractable_Event)))))

(fn ConstructionScript)