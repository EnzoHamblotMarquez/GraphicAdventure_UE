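; BP_AdventureCharacter is a character Blueprint that handles pausing and NPC dialogue states.
; Pause input opens UW_PauseMenu, switches to UI-only input and pauses the game.
; StartDialogue freezes movement, PlayTalkingPose cycles four montage sections by TalkIndex, and EndDialogue stops the montage and restores walking.
; OnNpcInteraction_Event triggers both dialogue start and pose, but its InteractionComponent binding is unconnected here.
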(event Custom|OnNpcInteraction_Event
  (CallFunction|StartDialogue)
  (CallFunction|PlayTalkingPose)
  (Development|PrintString "EVENT"))

(event Custom|Start%20Dialogue
  (Variables|Default|SetIsTalking true)
  (Components|Movement|StopMovementImmediately (Variables|Character|GetCharacterMovement))
  (Pawn|Components|CharacterMovement|DisableMovement (Variables|Character|GetCharacterMovement)))

(event Custom|PlayTalkingPose
  (switch int (Variables|Default|GetTalkIndex)
    (:0
      (Animation|Montage|PlayMontage (Variables|Character|GetMesh) "/Game/Animations/Secuences/Talking_Montage.Talking_Montage" 1.0 0.0 "Talk1"
        (:then
          (Variables|Default|SetTalkIndex (Math|Integer|%(Integer) (+ (Variables|Default|GetTalkIndex) 1) 4)))))
    (:1
      (Animation|Montage|PlayMontage (Variables|Character|GetMesh) "/Game/Animations/Secuences/Talking_Montage.Talking_Montage" 1.0 0.0 "Talk2"
        (:then
          (Variables|Default|SetTalkIndex (Math|Integer|%(Integer) (+ (Variables|Default|GetTalkIndex) 1) 4)))))
    (:2
      (Animation|Montage|PlayMontage (Variables|Character|GetMesh) "/Game/Animations/Secuences/Talking_Montage.Talking_Montage" 1.0 0.0 "Talk3"
        (:then
          (Variables|Default|SetTalkIndex (Math|Integer|%(Integer) (+ (Variables|Default|GetTalkIndex) 1) 4)))))
    (:3
      (Animation|Montage|PlayMontage (Variables|Character|GetMesh) "/Game/Animations/Secuences/Talking_Montage.Talking_Montage" 1.0 0.0 "Talk4"
        (:then
          (Variables|Default|SetTalkIndex (Math|Integer|%(Integer) (+ (Variables|Default|GetTalkIndex) 1) 4)))))))

(event Custom|EndDialogue
  (Variables|Default|SetIsTalking false)
  (Animation|Montage|MontageStop (Components|SkeletalMesh|GetAnimInstance (Variables|Character|GetMesh)) 0.0 "/Game/Animations/Secuences/Talking_Montage.Talking_Montage")
  (Pawn|Components|CharacterMovement|SetMovementMode (Variables|Character|GetCharacterMovement) "MOVE_Walking" 0))

(event Input|EnhancedActionEvents|EnhancedInputActionIA_Pause
  (params (ActionValue :type Boolean) (ElapsedSeconds :type Float%20%28double-precision%29) (TriggeredSeconds :type Float%20%28double-precision%29) (InputAction :type Input%20Action%20Object%20Reference :default "/Game/Inputs/Actions/IA_Pause.IA_Pause"))
  (bind _returnvalue (Game|GetPlayerController 0))
  (:Started
    (bind _returnvalue_2 (UserInterface|CreateWidget "/Game/Blueprints/UW/UW_PauseMenu.UW_PauseMenu_C"))
    (UserInterface|Viewport|AddtoViewport _returnvalue_2 0)
    (Variables|/Script/Engine.PlayerController|SetbShowMouseCursor _returnvalue true)
    (Input|SetInputModeUIOnly _returnvalue 0 "DoNotLock" false)
    (Game|SetGamePaused true)))

(event EventBeginPlay
  (Input|SetInputModeGameOnly (Game|GetPlayerController 0) false)
  (Variables|Default|SetIsTalking false))

(fn ConstructionScript)