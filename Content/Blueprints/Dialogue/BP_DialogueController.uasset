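; Dialogue controller that steps through data-table-driven NPC conversations each time the player's InteractionComponent fires OnNpcInteraction.
; The first interaction creates UW_Dialogue with UI-only input and calls EndDialogue on BP_AdventureCharacter; later ones update the text and play the talking pose.
; Each row supplies the next row, table and end flag, so conversations chain across tables.
; A set end flag makes the following interaction remove the widget and restore game input.
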(event Custom|OnNpcInteraction_Event
  (bind _returnvalue (Game|GetPlayerController 0))
  (Utilities|FlowControl|Sequence
    (:then_1
      (if (Variables|Default|GetEnddialogue)
        (Widget|RemovefromParent (Variables|Default|GetDialoguewidget))
        (Variables|Default|SetEnddialogue false)
        (Variables|Default|SetDialoguewidget 0)
        (Input|SetInputModeGameOnly _returnvalue true)
        (else
          (Utilities|IsValid (Variables|Default|GetDialoguewidget)
            (:Is%20Valid
              (bind _returnvalue_2 (Utilities|GetDataTableRow (Variables|Default|GetData%20Table) (Variables|Default|GetRow%20Name))
                (:then
                  (bind _asbp_adventure_character (Utilities|Casting|CastToBP_AdventureCharacter (Game|GetPlayerCharacter 0)))
                  (Default|PlayTalkingPose _asbp_adventure_character)
                  (Default|UpdateDialogue (Variables|Default|GetDialoguewidget) (.Dialogue (Utilities|Struct|BreakDialogue_Structure _returnvalue_2)) (Utilities|Text|ToText(Name) (Variables|Default|GetName)))
                  (Variables|Default|SetRow%20Name (.Row (Utilities|Struct|BreakDialogue_Structure _returnvalue_2)))
                  (Variables|Default|SetData%20Table (.Datatable (Utilities|Struct|BreakDialogue_Structure _returnvalue_2)))
                  (Variables|Default|SetEnddialogue (.EndDialogue? (Utilities|Struct|BreakDialogue_Structure _returnvalue_2))))))
            (:Is%20Not%20Valid
              (bind _returnvalue_3 (Utilities|GetDataTableRow (Variables|Default|GetData%20Table) (Variables|Default|GetRow%20Name))
                (:then
                  (bind _returnvalue_4 (UserInterface|CreateWidget "/Game/Blueprints/Dialogue/UW_Dialogue.UW_Dialogue_C" 0 (Utilities|Text|ToText(Name) (Variables|Default|GetName)) (.Dialogue (Utilities|Struct|BreakDialogue_Structure _returnvalue_3))))
                  (bind _output_get (Variables|Default|SetDialoguewidget _returnvalue_4))
                  (UserInterface|Viewport|AddtoViewport _output_get 0)
                  (Input|SetInputModeUIOnly _returnvalue _output_get "DoNotLock" true)
                  (Variables|/Script/Engine.PlayerController|SetbShowMouseCursor _returnvalue false) ; NOT WORKING
                  (Variables|Default|SetRow%20Name (.Row (Utilities|Struct|BreakDialogue_Structure _returnvalue_3)))
                  (Variables|Default|SetData%20Table (.Datatable (Utilities|Struct|BreakDialogue_Structure _returnvalue_3)))
                  (Variables|Default|SetEnddialogue (.EndDialogue? (Utilities|Struct|BreakDialogue_Structure _returnvalue_3)))
                  (bind _asbp_adventure_character_2 (Utilities|Casting|CastToBP_AdventureCharacter (Game|GetPlayerCharacter 0)))
                  (Default|EndDialogue _asbp_adventure_character_2))))))))))

(event EventBeginPlay
  (EventDispatchers|AssignOnNpcInteraction (Actor|GetComponentbyClass (Game|GetPlayerCharacter 0) "/Script/GraphicAdventure_UE.InteractionComponent") (delegate Custom|OnNpcInteraction_Event))
  (Variables|Default|SetDialoguewidget 0)
  (Variables|Default|SetRow%20Name "1"))

(fn ConstructionScript)